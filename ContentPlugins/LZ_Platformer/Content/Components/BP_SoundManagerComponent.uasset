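; Sound manager component that plays 2D sound effects for a BP_BetterJumperStates owner and starts the forest ambience.
; On BeginPlay it casts its owner and binds to the state change, fall, respawn and jump events.
; Each jump type picks a sound, with air and wall jumps sharing one, followed by a whoosh.
; Wall slides, falls and respawns trigger their own sounds, and Tick is unused.
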(event Custom|State%20Changed%20Event
  (params (Prev%20State :type ENUM_LZ_PlatformerStates%20Enum :default "NewEnumerator0") (New%20State :type ENUM_LZ_PlatformerStates%20Enum :default "NewEnumerator0"))
  (switch Utilities|FlowControl|Switch|SwitchonENUM_LZ_PlatformerStates New%20State
    (:NewEnumerator4
      (Audio|PlaySound2D "/Game/Developers/Pasha/Assets/MetaBoy/Sounds/EarthCling.EarthCling" 0.75 1.0 0.0 0 0))))

(event Custom|OnFallEvent
  (Audio|PlaySound2D "/Game/Developers/Pasha/Assets/MetaBoy/Sounds/FallDeath.FallDeath" 1.0 1.0 0.0 0 0))

(event Custom|OnRespawn
  (Audio|PlaySound2D "/Game/Developers/Pasha/Assets/MetaBoy/Sounds/WhooshFast_Cue.WhooshFast_Cue" 1.0 1.0 0.0 0 0))

(event Custom|OnJump
  (params (JumpType :type ENUM_LZ_JumpTypes%20Enum :default "NewEnumerator0"))
  (switch Utilities|FlowControl|Switch|SwitchonENUM_LZ_JumpTypes JumpType
    (:NewEnumerator0
      (Audio|PlaySound2D "/Game/Developers/Pasha/Assets/MetaBoy/Sounds/JumpAir.JumpAir" 1.0 1.0 0.0 0 0))
    (:NewEnumerator2
      (Audio|PlaySound2D "/Game/Developers/Pasha/Assets/MetaBoy/Sounds/Yes.Yes" 1.0 1.0 0.0 0 0 :!label _label))
    (:NewEnumerator1
      (Audio|PlaySound2D "/Game/Developers/Pasha/Assets/MetaBoy/Sounds/Jump3.Jump3" 1.0 1.0 0.0 0 0))
    (:NewEnumerator3
      (Audio|PlaySound2D "/Game/Developers/Pasha/Assets/MetaBoy/Sounds/haha.haha" 1.0 1.0 0.0 0 0))
    (:NewEnumerator4
      (goto _label)))
  (Audio|PlaySound2D "/Game/Developers/Pasha/Assets/MetaBoy/Sounds/WhooshFast_Cue.WhooshFast_Cue" 1.0 1.0 0.0 0 0))

(event EventBeginPlay
  (bind _asbp_better_jumper_states (Utilities|Casting|CastToBP_BetterJumperStates (Components|GetOwner)))
  (bind _output_get (Variables|Default|SetOwner _asbp_better_jumper_states))
  (EventDispatchers|BindEventtoStateChangedEvent _output_get (delegate Custom|State%20Changed%20Event))
  (EventDispatchers|BindEventtoFallEvent _output_get (delegate Custom|OnFallEvent))
  (EventDispatchers|BindEventtoRespawnEvent (Variables|Default|GetOwner) (delegate Custom|OnRespawn))
  (EventDispatchers|BindEventtoJumpEvent (Variables|Default|GetOwner) (delegate Custom|OnJump))
  (Audio|PlaySound2D "/Game/Developers/Pasha/Assets/MetaBoy/Sounds/Ambient/ForestAmbient.ForestAmbient" 1.0 1.0 0.0 0 0 false :!pinned true) ; Ambient Sound
)

(event EventTick
  (params (DeltaSeconds :type Float%20%28single-precision%29)))