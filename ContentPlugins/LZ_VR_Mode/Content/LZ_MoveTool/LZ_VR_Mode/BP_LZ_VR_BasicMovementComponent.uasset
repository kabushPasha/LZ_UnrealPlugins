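; VR movement component for an XRCreativeAvatar owner, providing grab-the-world drag, rotate and scale locomotion from Enhanced Input actions.
; One-hand drag caches grip and avatar transforms, then moves the avatar by the inverse grip delta; right-hand drag yields while IsDraggingActor is set.
; Two-hand gesture stops dragging, moves the avatar by the dual-grip delta, and rescales WorldToMeters by controller-distance ratio, updating child component scale through BPI_XRC_Movement.
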(event Custom|StopMoveDrag
  (Utilities|HandleDragMovementLZ "Left") ; enters at Stop
)

(event Custom|Initialize
  (bind _asxrcreative_avatar (Utilities|Casting|CastToXRCreativeAvatar (Components|GetOwner)))
  (bind _output_get (Variables|Default|SetOwnerAvatar _asxrcreative_avatar))
  (bind _asbpi_xrc_movement (Utilities|Casting|CastToBPI_XRC_Movement _output_get))
  (Variables|Default|SetOwner%20BPI%20XRC%20Movement _asbpi_xrc_movement))

(event Input|EnhancedActionEvents|EnhancedInputActionIA_RotateAndScale
  (params (ActionValue :type Boolean) (ElapsedSeconds :type Float%20%28double-precision%29) (TriggeredSeconds :type Float%20%28double-precision%29) (InputAction :type Input%20Action%20Object%20Reference :default "/VirtualScouting/Input/IA_RotateAndScale.IA_RotateAndScale"))
  (:Triggered
    (goto _label Start))
  (:Canceled
    (Utilities|HandleTwoHandedRotateandScaleLZ :!label _label))
  (:Completed
    (goto _label)))

(event Input|EnhancedActionEvents|EnhancedInputActionIA_DragLeft
  (params (ActionValue :type Boolean) (ElapsedSeconds :type Float%20%28double-precision%29) (TriggeredSeconds :type Float%20%28double-precision%29) (InputAction :type Input%20Action%20Object%20Reference :default "/VirtualScouting/Input/IA_DragLeft.IA_DragLeft"))
  (:Triggered
    (Utilities|HandleDragMovementLZ "Left" :!label _label))
  (:Canceled
    (goto _label Stop))
  (:Completed
    (goto _label Stop)))

(event Input|EnhancedActionEvents|EnhancedInputActionIA_DragRight
  (params (ActionValue :type Boolean) (ElapsedSeconds :type Float%20%28double-precision%29) (TriggeredSeconds :type Float%20%28double-precision%29) (InputAction :type Input%20Action%20Object%20Reference :default "/VirtualScouting/Input/IA_DragRight.IA_DragRight"))
  (:Triggered
    (Utilities|HandleDragMovementLZ "Right" :!label _label))
  (:Canceled
    (goto _label Stop))
  (:Completed
    (goto _label Stop)))

(event EventTick
  (params (DeltaSeconds :type Float%20%28single-precision%29)))