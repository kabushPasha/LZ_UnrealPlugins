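; Actor component on a player Character that runs the pause menu and adds the controller UI input mapping context.
; The pause input lazily creates the menu widget and binds its Continue, Main Menu and Quit buttons through an interface.
; A shared Pause toggle, also reached by Continue and UI Back while paused, switches widget visibility, game pause, input mode and sound.
; The mouse cursor appears only when keyboard and mouse was the last-used device.
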(event Custom|PauseClicked
  (CallFunction|Pause))

(event Custom|Quit
  (Game|QuitGame 0 "Quit" false))

(event Custom|Main%20Menu
  (Game|OpenLevel(byObjectReference) (Variables|Default|GetMain%20Menu%20Map)))

(event Input|EnhancedActionEvents|EnhancedInputActionIA_Pause
  (params (ActionValue :type Boolean) (ElapsedSeconds :type Float%20%28double-precision%29) (TriggeredSeconds :type Float%20%28double-precision%29) (InputAction :type Input%20Action%20Object%20Reference :default "/LZ_BasicUI/Logic/Input/IA_Pause.IA_Pause"))
  (:Completed
    (Utilities|IsValid (Utilities|ToObject(Interface) (Variables|Default|GetAs%20BPI%20Pause%20Menu))
      (:Is%20Valid
        _)
      (:Is%20Not%20Valid
        (bind _returnvalue (UserInterface|CreateWidget (Variables|Default|GetPause%20Menu%20Widget%20Class)))
        (bind _output_get (Variables|Default|SetPause%20Menu%20Widget _returnvalue))
        (bind _asbpi_get_basic_buttons (Utilities|Casting|CastToBPI_GetBasicButtons _output_get))
        (bind _output_get_2 (Variables|Default|SetAs%20BPI%20Pause%20Menu _asbpi_get_basic_buttons))
        (bind (_continue _mainmenu _quit) (Default|GetButtons _output_get_2))
        (EventDispatchers|BindEventtoOnClicked _continue (delegate Custom|PauseClicked))
        (EventDispatchers|BindEventtoOnClicked _mainmenu (delegate Custom|Main%20Menu))
        (EventDispatchers|BindEventtoOnClicked _quit (delegate Custom|Quit))))
    (CallFunction|Pause)))

(event Input|EnhancedActionEvents|EnhancedInputActionIA_UI_Back
  (params (ActionValue :type Boolean) (ElapsedSeconds :type Float%20%28double-precision%29) (TriggeredSeconds :type Float%20%28double-precision%29) (InputAction :type Input%20Action%20Object%20Reference :default "/LZ_BasicUI/Logic/Input/IA_UI_Back.IA_UI_Back"))
  (if (Game|IsGamePaused)
    (CallFunction|Pause)))

(event EventBeginPlay
  (bind _ascharacter (Utilities|Casting|CastToCharacter (Components|GetOwner)))
  (bind _asplayer_controller (Utilities|Casting|CastToPlayerController (Pawn|GetController _ascharacter)))
  (Input|AddMappingContext (PlayerController|LocalPlayerSubsystems|GetEnhancedInputLocalPlayerSubsystem _asplayer_controller) "/LZ_BasicUI/Logic/Input/IMC_ControllerUI.IMC_ControllerUI" 0 "(bIgnoreAllPressedKeysUntilRelease=True,bForceImmediately=False,bNotifyUserSettings=False)"))

(event EventTick
  (params (DeltaSeconds :type Float%20%28single-precision%29)))

(fn Pause
  (bind _returnvalue (Game|GetPlayerController 0))
  (bind _returnvalue_2 (Game|GetPlayerController 0))
  (bind _pause_menu_widget (Variables|Default|GetPause%20Menu%20Widget))
  (if (Game|IsGamePaused)
    (Widget|RemovefromParent _pause_menu_widget)
    (Game|SetGamePaused false)
    (Variables|/Script/Engine.PlayerController|SetbShowMouseCursor _returnvalue_2 false)
    (Input|SetInputModeGameOnly _returnvalue_2 false)
    (Audio|PlaySound2D (Variables|Default|GetPauseCloseSFX) 1.0 1.0 0.0 0 0)
    (else
      (UserInterface|Viewport|AddtoViewport _pause_menu_widget 0)
      (Game|SetGamePaused true)
      (Variables|/Script/Engine.PlayerController|SetbShowMouseCursor _returnvalue (Utilities|Enum|Equal(Enum) (.primarydevicetype (Class|InputDeviceSubsystem|GetMostRecentlyUsedHardwareDevice (|InputDeviceSubsystem))) "KeyboardAndMouse"))
      (Input|SetInputModeGameandUI _returnvalue 0 "DoNotLock" true true)
      (Audio|PlaySound2D (Variables|Default|GetPauseOpenSFX) 1.0 1.0 0.0 0 0))))