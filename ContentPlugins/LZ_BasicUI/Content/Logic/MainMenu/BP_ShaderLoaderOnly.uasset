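; Startup Blueprint that shows a shader compilation loading screen, then opens the MainMenu level.
; BeginPlay constructs the ShaderLoader class through BPI_ProgressTask and seeds WB_ShaderCompileLoad's maximum with its initial progress count.
; Tick polls that count as remaining work, updating the widget until it reaches zero or below, then removes it and loads the menu.
; An invalid or non-implementing loader class skips straight to the menu.
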(event Custom|AllShadersLoaded
  (Game|OpenLevel(byObjectReference) (Variables|Default|GetMainMenu)))

(event EventBeginPlay
  (bind _shaderloader (Variables|Default|GetShaderLoader))
  ;[0.15 0.15 0.15 0.5] BeginPlay : Show Shader Loading Screen and pick Loader
  (if (and (Utilities|IsValidClass _shaderloader) (Class|KismetSystemLibrary|DoesClassImplementInterface _shaderloader "/LZ_BasicUI/Logic/MainMenu/ProgressTask/BPI_ProgressTask.BPI_ProgressTask_C"))
    (bind _returnvalue (Game|ConstructObjectfromClass (Variables|Default|GetShaderLoader)))
    (bind _asbpi_progress_task (Utilities|Casting|CastToBPI_ProgressTask _returnvalue))
    (Variables|Default|SetShader%20Loader%20Progress%20Task _asbpi_progress_task)
    (bind _returnvalue_2 (UserInterface|CreateWidget (Variables|Default|GetShader%20CompilerWidget)))
    (bind _aswb_shader_compile_load (Utilities|Casting|CastToWB_ShaderCompileLoad _returnvalue_2))
    (bind _output_get (Variables|Default|SetWB%20Shader%20Compiler _aswb_shader_compile_load))
    (UserInterface|Viewport|AddtoViewport _output_get 0)
    (Variables|Default|SetShadersCompiled false)
    (bind _progress (Default|GetProgress (Variables|Default|GetShader%20Loader%20Progress%20Task)))
    (Variables|/LZ_BasicUI/UI/Widgets/ShaderCompiler/WB_ShaderCompileLoad.WB_ShaderCompileLoad_C|SetMax_shaders _output_get _progress)
    (else
      (CallFunction|AllShadersLoaded)
      (Variables|Default|SetShadersCompiled true))))

(event EventTick
  (params (DeltaSeconds :type Float%20%28single-precision%29))
  (bind _wb_shader_compiler (Variables|Default|GetWB%20Shader%20Compiler))
  ;[0.15 0.15 0.15 0.5] Tick : check if we're compiling Shaders
  (if (not (Variables|Default|GetShadersCompiled))
    (bind _progress (Default|GetProgress (Variables|Default|GetShader%20Loader%20Progress%20Task)))
    (Math|Integer|CompareInt _progress
      (:>
        (Default|SetProgress _wb_shader_compiler _progress))
      (:==
        (Variables|Default|SetShadersCompiled true :!label _label)
        (Widget|RemovefromParent _wb_shader_compiler)
        (CallFunction|AllShadersLoaded))
      (:<
        (goto _label)))))

(event Collision|EventActorBeginOverlap
  (params (OtherActor :type Actor%20Object%20Reference)))

(fn ConstructionScript)